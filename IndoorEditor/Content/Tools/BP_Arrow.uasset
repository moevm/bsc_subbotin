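; BP_Arrow is a translate-gizmo arrow that drags its owning actor along one axis with the mouse.
; Construction derives the axis index from the arrow's rotation and tints cylinder and cone red, green or blue through dynamic materials.
; Tick traces under the cursor; while clicked, the hit-point delta, masked to that axis, moves the hit arrow's owner and every BP_Arrow in the world.
; Releasing or leaving the arrow ends the drag.
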(event `self.ReceiveActorOnClicked`
  (params (ButtonPressed :type "Key Structure"))
  (set `self.mouseClicked` true))

(event `self.ReceiveActorOnReleased`
  (params (ButtonReleased :type "Key Structure"))
  (set `self.mouseClicked` false :!label _label))

(event `self.ReceiveActorEndCursorOver`
  (goto _label))

(event `self.ReceiveTick`
  (params (DeltaSeconds :type "Float (single-precision)"))
  (bind _toolnum (`self.toolNum`))
  (bind (_bblockinghit _binitialoverlap _time _distance _location _impactpoint _normal _impactnormal _physmat _hitactor) (`GameplayStatics.BreakHitResult` (`PlayerController.GetHitResultUnderCursorByChannel` (`GameplayStatics.GetPlayerController` 0) "TraceTypeQuery1" true)))
  (bind _returnvalue (`self.GetOwner` _hitactor))
  (bind _returnvalue_2 (`KismetMathLibrary.MakeVector` (* (.x (- _location (`self.startMousePoint`))) (`KismetMathLibrary.Conv_BoolToDouble` (== _toolnum 1))) (* (.y (- _location (`self.startMousePoint`))) (`KismetMathLibrary.Conv_BoolToDouble` (== _toolnum 2))) (* (.z (- _location (`self.startMousePoint`))) (`KismetMathLibrary.Conv_BoolToDouble` (== _toolnum 3)))))
  (cast `/Game/Tools/BP_Arrow` _hitactor
    (:`then`
      (if (`self.mouseClicked`)
        (`self.K2_SetActorLocation` _returnvalue (+ _returnvalue_2 (`self.K2_GetActorLocation` _returnvalue)) false false)
        (`self.newArrowPos` _returnvalue_2)
        (set `self.startMousePoint` _location)
        (else
          (set `self.startMousePoint` _location))))
    (:`CastFailed`
      (goto _label))))

(fn `getIndex`
  (bind _returnvalue (+ (`KismetMathLibrary.SelectInt` 2 0 (`KismetMathLibrary.NearlyEqual_FloatFloat` (.roll (`self.K2_GetActorRotation` self)) 90.0 0.0001)) (`KismetMathLibrary.SelectInt` 1 0 (`KismetMathLibrary.NearlyEqual_FloatFloat` (.pitch (`self.K2_GetActorRotation` self)) -90.0 0.0001))))
  ;[1 1 1] По углу поворота задаём индекс инструмента
  (set `self.toolNum` (`KismetMathLibrary.SelectInt` _returnvalue 3 (!= _returnvalue 0))))

(fn `newArrowPos`
  (params (offset :type "Vector Structure"))
  (bind _outactors (`GameplayStatics.GetAllActorsOfClass` "BP_Arrow_C"))
  (for _array_element _outactors
    (`self.K2_SetActorLocation` _array_element (+ (`self.K2_GetActorLocation` _array_element) offset) false false)))

(fn `UserConstructionScript`
  (bind _toolnum (`self.toolNum`))
  (bind _linearcolor (make `LinearColor` (`KismetMathLibrary.Conv_BoolToDouble` (== _toolnum 1)) (`KismetMathLibrary.Conv_BoolToDouble` (== _toolnum 2)) (`KismetMathLibrary.Conv_BoolToDouble` (== _toolnum 3))))
  (`self.getIndex`)
  (bind _returnvalue (`PrimitiveComponent.CreateDynamicMaterialInstance` (`self.Cylinder`) 0 "/Game/Materials/toolMaterial.toolMaterial" "None"))
  (`MaterialInstanceDynamic.SetVectorParameterValue` _returnvalue "toolColor" _linearcolor)
  (bind _returnvalue_2 (`PrimitiveComponent.CreateDynamicMaterialInstance` (`self.Cone`) 0 "/Game/Materials/toolMaterial.toolMaterial" "None"))
  (`MaterialInstanceDynamic.SetVectorParameterValue` _returnvalue_2 "toolColor" _linearcolor))