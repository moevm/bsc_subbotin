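; BP_Scale is a single-axis scale gizmo handle that resizes its owning actor when dragged with the mouse.
; Construction derives the X, Y or Z axis from the handle's rotation and colors its dynamic material red, green or blue.
; Tick traces under the cursor while pressed, adds axis-masked movement to the owner's absolute scale, then stretches and shifts the handle.
; Releasing or moving off the handle ends the drag.
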(event `self.ReceiveActorOnClicked`
  (params (ButtonPressed :type "Key Structure"))
  (set `self.mouseClicked` true))

(event `self.ReceiveActorOnReleased`
  (params (ButtonReleased :type "Key Structure"))
  (set `self.mouseClicked` false :!label _label))

(event `self.ReceiveActorEndCursorOver`
  (goto _label))

(event `self.ReceiveTick`
  (params (DeltaSeconds :type "Float (single-precision)"))
  (bind _toolnum (`self.toolNum`))
  (bind (_bblockinghit _binitialoverlap _time _distance _location _impactpoint _normal _impactnormal _physmat _hitactor) (`GameplayStatics.BreakHitResult` (`PlayerController.GetHitResultUnderCursorByChannel` (`GameplayStatics.GetPlayerController` 0) "TraceTypeQuery1" true)))
  (bind _returnvalue (`self.GetOwner` _hitactor))
  (bind _returnvalue_2 (`KismetMathLibrary.MakeVector` (* (.x (/ (- _location (`self.startMousePoint`)) 50)) (`KismetMathLibrary.Conv_BoolToDouble` (== _toolnum 1))) (* (.y (/ (- _location (`self.startMousePoint`)) 50)) (`KismetMathLibrary.Conv_BoolToDouble` (== _toolnum 2))) (* (.z (/ (- _location (`self.startMousePoint`)) 50)) (`KismetMathLibrary.Conv_BoolToDouble` (== _toolnum 3)))))
  (cast `/Game/Tools/BP_Scale` _hitactor
    (:`then`
      (if (`self.mouseClicked`)
        (`self.SetActorScale3D` _returnvalue (`KismetMathLibrary.Vector_GetAbs` (+ _returnvalue_2 (`self.GetActorScale3D` _returnvalue))))
        (`self.setScaleSize` _returnvalue_2)
        (set `self.startMousePoint` _location)
        (else
          (set `self.startMousePoint` _location))))
    (:`CastFailed`
      (goto _label))))

(fn `getIndex`
  (bind _returnvalue (+ (`KismetMathLibrary.SelectInt` 2 0 (`KismetMathLibrary.NearlyEqual_FloatFloat` (.roll (`self.K2_GetActorRotation` self)) 90.0 0.0001)) (`KismetMathLibrary.SelectInt` 1 0 (`KismetMathLibrary.NearlyEqual_FloatFloat` (.pitch (`self.K2_GetActorRotation` self)) -90.0 0.0001))))
  ;[1 1 1] По углу поворота задаём индекс инструмента
  (set `self.toolNum` (`KismetMathLibrary.SelectInt` _returnvalue 3 (!= _returnvalue 0))))

(fn `setScaleSize`
  (params (scaleVector :type "Vector Structure"))
  (bind _returnvalue (`KismetMathLibrary.Vector_GetAbsMax` scaleVector))
  (bind _cube (`self.Cube`))
  (`SceneComponent.SetWorldScale3D` _cube (`KismetMathLibrary.MakeVector` (.x (`SceneComponent.K2_GetComponentScale` _cube)) (.y (`SceneComponent.K2_GetComponentScale` _cube)) (+ (.z (`SceneComponent.K2_GetComponentScale` _cube)) (* _returnvalue (`KismetMathLibrary.SelectFloat` 1.0 -1.0 (`KismetMathLibrary.NearlyEqual_FloatFloat` (`KismetMathLibrary.GetMaxElement` scaleVector) _returnvalue 0.0001))))))
  (`self.K2_AddActorWorldOffset` (* scaleVector 50.0)))

(fn `UserConstructionScript`
  (bind _toolnum (`self.toolNum`))
  (`self.getIndex`)
  (bind _returnvalue (`PrimitiveComponent.CreateDynamicMaterialInstance` (`self.Cube`) 0 "/Game/Materials/toolMaterial.toolMaterial" "None"))
  (`MaterialInstanceDynamic.SetVectorParameterValue` _returnvalue "toolColor" (make `LinearColor` (`KismetMathLibrary.Conv_BoolToDouble` (== _toolnum 1)) (`KismetMathLibrary.Conv_BoolToDouble` (== _toolnum 2)) (`KismetMathLibrary.Conv_BoolToDouble` (== _toolnum 3)))))