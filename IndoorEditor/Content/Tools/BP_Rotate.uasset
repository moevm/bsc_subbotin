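; Rotation gizmo handle that turns its owner actor around one world axis when dragged with the mouse.
; Construction infers the axis (ToolNum) from the handle's own orientation and tints the cylinder red, green or blue to match.
; While held, Tick traces under the cursor, derives the per-frame angle by law of cosines, picks its sign and applies it.
; Releasing or moving the cursor off the handle ends the drag.
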(event `self.ReceiveActorOnClicked`
  (params (ButtonPressed :type "Key Structure"))
  (set `self.mouseClicked` true))

(event `self.ReceiveActorOnReleased`
  (params (ButtonReleased :type "Key Structure"))
  (set `self.mouseClicked` false :!label _label))

(event `self.ReceiveActorEndCursorOver`
  (goto _label))

(event `self.ReceiveTick`
  (params (DeltaSeconds :type "Float (single-precision)"))
  (bind _startmousepoint (`self.startMousePoint`))
  (bind _toolnum (`self.toolNum`))
  (bind _returnvalue (== _toolnum 1))
  (bind _returnvalue_2 (== _toolnum 2))
  (bind _returnvalue_3 (== _toolnum 3))
  (bind (_bblockinghit _binitialoverlap _time _distance _location _impactpoint _normal _impactnormal _physmat _hitactor) (`GameplayStatics.BreakHitResult` (`PlayerController.GetHitResultUnderCursorByChannel` (`GameplayStatics.GetPlayerController` 0) "TraceTypeQuery1" true)))
  (bind _returnvalue_4 (`KismetMathLibrary.Conv_BoolToDouble` (not _returnvalue_3)))
  (bind _returnvalue_5 (`KismetMathLibrary.Conv_BoolToDouble` (not _returnvalue)))
  (bind _returnvalue_6 (`KismetMathLibrary.Conv_BoolToDouble` (not _returnvalue_2)))
  (bind _returnvalue_7 (`self.GetOwner` _hitactor))
  (bind _returnvalue_8 (`self.K2_GetActorLocation` _returnvalue_7))
  (bind _returnvalue_9 (* (.x (- _location _startmousepoint)) _returnvalue_5))
  (bind _returnvalue_10 (* (.y (- _location _startmousepoint)) _returnvalue_6))
  (bind _returnvalue_11 (* (.z (- _returnvalue_8 _startmousepoint)) _returnvalue_4))
  (bind _returnvalue_12 (* (.y (- _returnvalue_8 _startmousepoint)) _returnvalue_6))
  (bind _returnvalue_13 (+ (`KismetMathLibrary.Square` (* (.x (- _returnvalue_8 _location)) _returnvalue_5)) (`KismetMathLibrary.Square` (* (.y (- _returnvalue_8 _location)) _returnvalue_6)) (`KismetMathLibrary.Square` (* (.z (- _returnvalue_8 _location)) _returnvalue_4))))
  (bind _returnvalue_14 (+ (`KismetMathLibrary.Square` (* (.x (- _returnvalue_8 _startmousepoint)) _returnvalue_5)) (`KismetMathLibrary.Square` _returnvalue_12) (`KismetMathLibrary.Square` _returnvalue_11)))
  (bind _returnvalue_15 (`KismetMathLibrary.SelectFloat` 1.0 -1.0 (> (+ (* _returnvalue_9 _returnvalue_12) (* _returnvalue_9 _returnvalue_11) (* _returnvalue_10 _returnvalue_11 -1.0)) 0.0)))
  (bind _returnvalue_16 (`KismetMathLibrary.DegAcos` (/ (- (+ _returnvalue_13 _returnvalue_14) (+ (`KismetMathLibrary.Square` _returnvalue_9) (`KismetMathLibrary.Square` _returnvalue_10) (`KismetMathLibrary.Square` (* (.z (- _location _startmousepoint)) _returnvalue_4)))) (* (`KismetMathLibrary.Sqrt` _returnvalue_13) (`KismetMathLibrary.Sqrt` _returnvalue_14) 2.0))))
  (cast `/Game/Tools/BP_Rotate` _hitactor
    (:`then`
      (if (`self.mouseClicked`)
        (`self.K2_AddActorWorldRotation` _returnvalue_7 (`KismetMathLibrary.MakeRotator` (* _returnvalue_16 (`KismetMathLibrary.Conv_BoolToDouble` _returnvalue) _returnvalue_15) (* _returnvalue_16 (`KismetMathLibrary.Conv_BoolToDouble` _returnvalue_2) _returnvalue_15) (* _returnvalue_16 (`KismetMathLibrary.Conv_BoolToDouble` _returnvalue_3) _returnvalue_15)) false false)
        (set `self.startMousePoint` _location)
        (else
          (set `self.startMousePoint` _location))))
    (:`CastFailed`
      (goto _label))))

(fn `getIndex`
  (bind _returnvalue (+ (`KismetMathLibrary.SelectInt` 2 0 (`KismetMathLibrary.NearlyEqual_FloatFloat` (.roll (`self.K2_GetActorRotation` self)) 90.0 0.0001)) (`KismetMathLibrary.SelectInt` 1 0 (`KismetMathLibrary.NearlyEqual_FloatFloat` (.pitch (`self.K2_GetActorRotation` self)) -90.0 0.0001))))
  ;[1 1 1] По углу поворота задаём индекс инструмента
  (set `self.toolNum` (`KismetMathLibrary.SelectInt` _returnvalue 3 (!= _returnvalue 0))))

(fn `UserConstructionScript`
  (bind _toolnum (`self.toolNum`))
  (`self.getIndex`)
  (bind _returnvalue (`PrimitiveComponent.CreateDynamicMaterialInstance` (`self.Cylinder`) 0 "/Game/Materials/toolMaterial.toolMaterial" "None"))
  (`MaterialInstanceDynamic.SetVectorParameterValue` _returnvalue "toolColor" (make `LinearColor` (`KismetMathLibrary.Conv_BoolToDouble` (== _toolnum 1)) (`KismetMathLibrary.Conv_BoolToDouble` (== _toolnum 2)) (`KismetMathLibrary.Conv_BoolToDouble` (== _toolnum 3)))))