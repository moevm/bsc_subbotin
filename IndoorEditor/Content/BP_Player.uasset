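; Player pawn for an in-game scene editor, with a fly camera, mouse selection of static meshes and Tab cycling through lights.
; Selection spawns three axis gizmos (move, scale or rotate) owned by the actor and rebuilds its settings widget.
; Hotkeys toggle gravity, delete, hide UI for screenshots, open the menu, and temporarily simulate physics on gravity-enabled meshes while Z is held.
; Scene states are saved into the SaveScene slot.
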(event `Key|G`
  (params (Key :type "Key Structure"))
  ;[1 1 1] Включаем/выключаем гравитацию для выбранного объекта
  (:`Pressed`
    (bind _asstatic_mesh_actor (cast `StaticMeshActor` (`self.currentActor`)))
    (bind _staticmeshcomponent (`StaticMeshActor.StaticMeshComponent` _asstatic_mesh_actor))
    (`PrimitiveComponent.SetEnableGravity` _staticmeshcomponent (not (`PrimitiveComponent.IsGravityEnabled` _staticmeshcomponent)))
    (`/Game/UI/ActorSettingsWB.GravityRefresh` (`self.settingsWB`))))

(event `Key|Tab`
  (params (Key :type "Key Structure"))
  ;[1 1 1] Выбор следующего источника света
  (:`Pressed`
    (bind _result (`/Engine/EditorBlueprintResources/StandardMacros.IncrementInt` (`self.currentLightIndex`))
      (:`  `
        (if (== (- (`KismetArrayLibrary.Array_Length` (`self.lightArray`)) _result) 0)
          (set `self.currentLightIndex` 0))
        (set `self.currentActor` (`|GetArrayItem` (`self.lightArray`) (`self.currentLightIndex`)))
        (`self.RefreshTools`)))))

(event `RefreshTools`
  (bind _settingswb (`self.settingsWB`))
  ;[1 1 1] Перезагрузка инструментария
  (`self.removeTools`)
  (`self.spawnTools` (`self.currentActor`))
  (`/Engine/EditorBlueprintResources/StandardMacros.IsValid` _settingswb
    (:`Is Valid`
      (`Widget.RemoveFromParent` _settingswb))
    (:`Is Not Valid`
      _))
  (bind _returnvalue (`|CreateWidget` "/Game/UI/ActorSettingsWB.ActorSettingsWB_C" null (`self.currentActor`) self))
  (`UserWidget.AddToViewport` _returnvalue 0)
  (set `self.settingsWB` _returnvalue))

(event `Key|X`
  (params (Key :type "Key Structure"))
  (bind _spawnmenuwb (`self.spawnMenuWB`))
  (bind _settingswb (`self.settingsWB`))
  ;[1 1 1] Переключение в режим скриншота
  (:`Pressed`
    (bind _output_get (set `self.screenMode` (not (`self.screenMode`))))
    (if _output_get
      (`self.removeTools`)
      (`/Engine/EditorBlueprintResources/StandardMacros.IsValid` _spawnmenuwb
        (:`Is Valid`
          (`Widget.RemoveFromParent` _spawnmenuwb))
        (:`Is Not Valid`
          _))
      (`/Engine/EditorBlueprintResources/StandardMacros.IsValid` _settingswb
        (:`Is Valid`
          (`Widget.RemoveFromParent` _settingswb)))
      (else
        (`self.AddSpawnMenu`)))))

(event `SaveGameToSlot`
  (params (saveStateSlot :type "/Game/Save/saveStateStructure Structure"))
  ;[1 1 1] Сохранение сцены
  (bind _returnvalue (`GameplayStatics.DoesSaveGameExist` "SaveScene"))
  (if _returnvalue
    (bind _returnvalue_2 (`GameplayStatics.LoadGameFromSlot` "SaveScene"))
    (bind _assave_game_bp (cast `/Game/Save/SaveGame_BP` _returnvalue_2))
    (`KismetArrayLibrary.Array_Insert` (`/Game/Save/SaveGame_BP.saveStateStructureArray` _assave_game_bp) saveStateSlot)
    (bind _returnvalue_3 (`GameplayStatics.SaveGameToSlot` _assave_game_bp "SaveScene"))
    (if _returnvalue_3
      (`Widget.RemoveFromParent` (`self.saveWB`) :!label _label)
      (bind _returnvalue_4 (`|CreateWidget` "/Game/UI/MainMenuWB.MainMenuWB_C" null self))
      (`UserWidget.AddToViewport` _returnvalue_4 0))
    (else
      (bind _returnvalue_5 (`GameplayStatics.CreateSaveGameObject` "/Game/Save/SaveGame_BP.SaveGame_BP_C"))
      (`KismetArrayLibrary.Array_Insert` (`/Game/Save/SaveGame_BP.saveStateStructureArray` _returnvalue_5) saveStateSlot)
      (bind _returnvalue_6 (`GameplayStatics.SaveGameToSlot` _returnvalue_5 "SaveScene"))
      (if _returnvalue_6
        (goto _label)))))

(event `Key|Q`
  (params (Key :type "Key Structure"))
  (bind _spawnmenuwb (`self.spawnMenuWB`))
  (bind _settingswb (`self.settingsWB`))
  ;[1 1 1] Переход в меню
  (:`Pressed`
    (`self.removeTools` :!label _label_2)
    (`/Engine/EditorBlueprintResources/StandardMacros.IsValid` _settingswb
      (:`Is Valid`
        (`Widget.RemoveFromParent` _settingswb))
      (:`Is Not Valid`
        _))
    (`/Engine/EditorBlueprintResources/StandardMacros.IsValid` _spawnmenuwb
      (:`Is Valid`
        (`Widget.RemoveFromParent` _spawnmenuwb)
        (bind _returnvalue (`|CreateWidget` "/Game/UI/MainMenuWB.MainMenuWB_C" null self))
        (`UserWidget.AddToViewport` _returnvalue 0)
        (`GameplayStatics.SetGamePaused` true)))))

(event `Key|Escape`
  (params (Key :type "Key Structure"))
  ;[1 1 1] Переход в меню
  (:`Pressed`
    (goto _label_2)))

(event `Key|Delete`
  (params (Key :type "Key Structure"))
  (bind _settingswb (`self.settingsWB`))
  ;[1 1 1] Удаляет модель
  (:`Pressed`
    (`self.removeTools`)
    (`/Engine/EditorBlueprintResources/StandardMacros.IsValid` _settingswb
      (:`Is Valid`
        (`Widget.RemoveFromParent` _settingswb)
        (`self.K2_DestroyActor` (`self.currentActor`))))))

(event `Key|Z`
  (params (Key :type "Key Structure"))
  (bind _settingswb (`self.settingsWB`))
  ;[1 1 1] Временно включаем физику для объектов
  (:`Pressed`
    (`/Engine/EditorBlueprintResources/StandardMacros.IsValid` _settingswb
      (:`Is Valid`
        (`Widget.RemoveFromParent` _settingswb)
        (`self.removeTools`)
        (bind _outactors (`GameplayStatics.GetAllActorsOfClass` "/Script/Engine.StaticMeshActor"))
        (for _array_element _outactors
          (bind _asstatic_mesh_actor (cast `StaticMeshActor` _array_element))
          (bind _staticmeshcomponent (`StaticMeshActor.StaticMeshComponent` _asstatic_mesh_actor))
          (if (`PrimitiveComponent.IsGravityEnabled` _staticmeshcomponent)
            (`PrimitiveComponent.SetSimulatePhysics` _staticmeshcomponent true))))))
  (:`Released`
    (bind _outactors_2 (`GameplayStatics.GetAllActorsOfClass` "/Script/Engine.StaticMeshActor"))
    (for _array_element_2 _outactors_2
      (bind _asstatic_mesh_actor_2 (cast `StaticMeshActor` _array_element_2))
      (`PrimitiveComponent.SetSimulatePhysics` (`StaticMeshActor.StaticMeshComponent` _asstatic_mesh_actor_2) false))))

(event `AddSpawnMenu`
  ;[1 1 1] При запуске программы предоставляется доступ к курсору и создаётся виджет спавна
  (bind _returnvalue (`|CreateWidget` "/Game/UI/SpawnMenuWB.SpawnMenuWB_C" null self :!label _label_3))
  (`UserWidget.AddToViewport` _returnvalue 0)
  (set `self.spawnMenuWB` _returnvalue)
  (bind _returnvalue_2 (`GameplayStatics.GetActorOfClass` "/Script/Engine.DirectionalLight"))
  (`KismetArrayLibrary.Array_Add` (`self.lightArray`) _returnvalue_2))

(event `self.ReceiveBeginPlay`
  (bind _returnvalue (`GameplayStatics.GetPlayerController` 0))
  ;[1 1 1] При запуске программы предоставляется доступ к курсору и создаётся виджет спавна
  (set `PlayerController.bEnableClickEvents` true _returnvalue)
  (set `PlayerController.bShowMouseCursor` true _returnvalue)
  (goto _label_3))

(event `Key|LeftMouseButton`
  (params (Key :type "Key Structure"))
  (bind (_hitresult _returnvalue) (`PlayerController.GetHitResultUnderCursorByChannel` (`GameplayStatics.GetPlayerController` 0) "TraceTypeQuery1" true))
  (bind (_bblockinghit _binitialoverlap _time _distance _location _impactpoint _normal _impactnormal _physmat _hitactor) (`GameplayStatics.BreakHitResult` _hitresult))
  ;[1 1 1] При нажатии кнопки мыши выбираем объект, при отпускании создаём инструменты и вызываем виджет
  (:`Pressed`
    (if _returnvalue
      (`/Engine/EditorBlueprintResources/StandardMacros.IsValid` (`self.GetOwner` _hitactor)
        (:`Is Not Valid`
          (bind _asstatic_mesh_actor (cast `StaticMeshActor` _hitactor))
          (set `self.currentActor` _asstatic_mesh_actor)))))
  (:`Released`
    (`/Engine/EditorBlueprintResources/StandardMacros.IsValid` (`self.currentActor`)
      (:`Is Valid`
        (`self.RefreshTools`)))))

(event `self.ReceiveTick`
  (params (DeltaSeconds :type "Float (single-precision)"))
  (bind _camera (`self.Camera`))
  (bind (_locationx _locationy) (`WidgetLayoutLibrary.GetMousePositionScaledByDPI` (`GameplayStatics.GetPlayerController` 0)))
  (bind _returnvalue (/ (- (`self.mouseY`) _locationy) 5.0))
  ;[1 1 1] Смещение камеры
  (`self.K2_AddActorWorldOffset` self (* (+ (* (`SceneComponent.GetForwardVector` _camera) (`self.forvardMove`)) (* (`SceneComponent.GetRightVector` _camera) (`self.rightMove`))) 5) false false)
  ;[1 1 1] Поворот камеры
  (if (`self.rightButtonClicked`)
    (if (<= (`KismetMathLibrary.Abs` (+ (.pitch (`self.K2_GetActorRotation` self)) _returnvalue)) 90.0)
      (`SceneComponent.K2_AddRelativeRotation` (`self.Camera`) (`KismetMathLibrary.MakeRotator` 0.0 _returnvalue (/ (- _locationx (`self.mouseX`)) 5.0)) false false)
      (set `self.mouseX` _locationx)
      (set `self.mouseY` _locationy))))

(event `Key|T`
  (params (Key :type "Key Structure"))
  (bind _currentactor (`self.currentActor`))
  ;[1 1 1] Управление объектом
  (:`Pressed`
    (`self.removeTools`)
    (`/Engine/EditorBlueprintResources/StandardMacros.IsValid` _currentactor
      (:`Is Valid`
        (set `self.currentClass` "/Game/Tools/BP_Arrow.BP_Arrow_C")
        (`self.spawnTools` _currentactor)))))

(event `Key|M`
  (params (Key :type "Key Structure"))
  (bind _currentactor (`self.currentActor`))
  ;[1 1 1] Управление объектом
  (:`Pressed`
    (`self.removeTools`)
    (`/Engine/EditorBlueprintResources/StandardMacros.IsValid` _currentactor
      (:`Is Valid`
        (set `self.currentClass` "/Game/Tools/BP_Scale.BP_Scale_C")
        (`self.spawnTools` _currentactor)))))

(event `Key|R`
  (params (Key :type "Key Structure"))
  (bind _currentactor (`self.currentActor`))
  ;[1 1 1] Управление объектом
  (:`Pressed`
    (`self.removeTools`)
    (`/Engine/EditorBlueprintResources/StandardMacros.IsValid` _currentactor
      (:`Is Valid`
        (set `self.currentClass` "/Game/Tools/BP_Rotate.BP_Rotate_C")
        (`self.spawnTools` _currentactor)))))

(event `Key|W`
  (params (Key :type "Key Structure"))
  ;[1 1 1] Управление камерой
  (:`Pressed`
    (set `self.forvardMove` 1))
  (:`Released`
    (set `self.forvardMove` 0)))

(event `Key|S`
  (params (Key :type "Key Structure"))
  ;[1 1 1] Управление камерой
  (:`Pressed`
    (set `self.forvardMove` -1))
  (:`Released`
    (set `self.forvardMove` 0)))

(event `Key|A`
  (params (Key :type "Key Structure"))
  ;[1 1 1] Управление камерой
  (:`Pressed`
    (set `self.rightMove` -1))
  (:`Released`
    (set `self.rightMove` 0)))

(event `Key|D`
  (params (Key :type "Key Structure"))
  ;[1 1 1] Управление камерой
  (:`Pressed`
    (set `self.rightMove` 1))
  (:`Released`
    (set `self.rightMove` 0)))

(event `Key|RightMouseButton`
  (params (Key :type "Key Structure"))
  (bind (_locationx _locationy) (`WidgetLayoutLibrary.GetMousePositionScaledByDPI` (`GameplayStatics.GetPlayerController` 0)))
  ;[1 1 1] Управление камерой
  (:`Pressed`
    (set `self.rightButtonClicked` true)
    (set `self.mouseX` _locationx)
    (set `self.mouseY` _locationy))
  (:`Released`
    (set `self.rightButtonClicked` false)))

(event `Key|SpaceBar`
  (params (Key :type "Key Structure"))
  (bind _camera (`self.Camera`))
  ;[1 1 1] Сброс накопленной погрешности по оси X
  (:`Pressed`
    (`SceneComponent.K2_SetRelativeRotation` _camera (`KismetMathLibrary.MakeRotator` (* (.roll (`SceneComponent.K2_GetComponentRotation` _camera)) 0.0) (.pitch (`SceneComponent.K2_GetComponentRotation` _camera)) (.yaw (`SceneComponent.K2_GetComponentRotation` _camera))) false false)))

(fn `removeTools`
  (bind _outactors (`GameplayStatics.GetAllActorsOfClass` (`self.currentClass`)))
  (for _array_element _outactors
    (`self.K2_DestroyActor` _array_element)))

(fn `spawnTools`
  (params (currentActor :type "Actor Object Reference"))
  (bind _returnvalue (`self.K2_GetActorLocation` currentActor))
  (bind _currentclass (`self.currentClass`))
  (bind _x (.x (`self.GetActorScale3D` currentActor)))
  (bind _y (.y (`self.GetActorScale3D` currentActor)))
  (bind _z (.z (`self.GetActorScale3D` currentActor)))
  (bind _returnvalue_2 (== (`self.currentClass`) "/Game/Tools/BP_Rotate.BP_Rotate_C"))
  (bind _returnvalue_3 (* (`KismetMathLibrary.FMax` _x _y) 1.5))
  (bind _returnvalue_4 (* (`KismetMathLibrary.FMax` _y _z) 1.5))
  (bind _returnvalue_5 (* (`KismetMathLibrary.FMax` _x _z) 1.5))
  (`|SpawnActorFromClass` _currentclass (`KismetMathLibrary.MakeTransform` _returnvalue (struct :`Pitch` -90.0) (`KismetMathLibrary.SelectVector` (`KismetMathLibrary.MakeVector` _returnvalue_4 _returnvalue_4 0.05) (`KismetMathLibrary.MakeVector` 1.0 1.0 _x) _returnvalue_2)) "Undefined" "OverrideRootScale" currentActor null)
  (`|SpawnActorFromClass` _currentclass (`KismetMathLibrary.MakeTransform` _returnvalue (struct :`Roll` 90.0) (`KismetMathLibrary.SelectVector` (`KismetMathLibrary.MakeVector` _returnvalue_5 _returnvalue_5 0.05) (`KismetMathLibrary.MakeVector` 1.0 1.0 _y) _returnvalue_2)) "Undefined" "OverrideRootScale" currentActor null)
  (`|SpawnActorFromClass` _currentclass (`KismetMathLibrary.MakeTransform` _returnvalue (struct) (`KismetMathLibrary.SelectVector` (`KismetMathLibrary.MakeVector` _returnvalue_3 _returnvalue_3 0.05) (`KismetMathLibrary.MakeVector` 1.0 1.0 _z) _returnvalue_2)) "Undefined" "OverrideRootScale" currentActor null))

(fn `UserConstructionScript`)